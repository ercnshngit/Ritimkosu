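; BP_ColorTile is a colored tile that can be switched between active and inactive states.
; On BeginPlay it picks a color material from its actor tag, defaulting to white, and applies it as a dynamic instance.
; Only tiles tagged White start active.
; ActivateTileBP and DeactivateTileBP events toggle the state, setting actor collision and an edge-size material parameter ("Kenar Boyutları").
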(event `self.ReceiveBeginPlay`
  (`|ExecutionSequence`
    (:`then_0`
      (if (`self.ActorHasTag` "Red")
        (set `self.MaterialColor` "/Game/Materials/MI_Red.MI_Red")
        (elif (`self.ActorHasTag` "Purple")
          (set `self.MaterialColor` "/Game/Materials/MI_Purple.MI_Purple")
          (elif (`self.ActorHasTag` "Blue")
            (set `self.MaterialColor` "/Game/Materials/MI_BLue.MI_Blue")
            (elif (`self.ActorHasTag` "Yellow")
              (set `self.MaterialColor` "/Game/Materials/MI_Yellow.MI_Yellow")
              (elif (`self.ActorHasTag` "Green")
                (set `self.MaterialColor` "/Game/Materials/MI_Green.MI_Green")
                (else
                  (set `self.MaterialColor` "/Game/Materials/MI_White.MI_White"))))))))
    (:`then_1`
      (bind _returnvalue (`KismetMaterialLibrary.CreateDynamicMaterialInstance` (`self.MaterialColor`)))
      (bind _output_get (set `self.Dynamic Mat` _returnvalue))
      (`PrimitiveComponent.SetMaterial` (`self.TileMesh`) 0 _output_get)
      (if (not (`self.ActorHasTag` "White"))
        (`self.Deactivating`)
        (else
          (`self.Activating`))))))

(event `self.ActivateTileBP`
  (`self.Activating`))

(event `self.DeactivateTileBP`
  (`self.Deactivating`))

(fn `Activating`
  (`self.SetActorEnableCollision` true)
  (`MaterialInstanceDynamic.SetScalarParameterValue` (`self.Dynamic Mat`) "Kenar Boyutları" 0.0))

(fn `Deactivating`
  (`self.SetActorEnableCollision` false)
  (`MaterialInstanceDynamic.SetScalarParameterValue` (`self.Dynamic Mat`) "Kenar Boyutları" 15.0))

(fn `UserConstructionScript`)