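; BP_RitimTile is a rhythm tile whose actor tag selects its color material and sound, with untagged tiles turning white but targeting the Red group.
; It starts deactivated; activation events toggle an edge-size parameter on its dynamic material, while collision stays enabled in both states.
; Play, not called within this Blueprint, checks that state: active plays the sound and activates every BP_ColorTile sharing the tag, inactive deactivates them.
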(event `self.ReceiveBeginPlay`
  (`|ExecutionSequence`
    (:`then_0`
      (if (`self.ActorHasTag` "Red")
        (set `self.RitimColor` "/Game/Materials/MI_Red.MI_Red")
        (set `self.Sound` "/Game/Sounds/S_Kick.S_Kick")
        (set `self.Tag` "Red")
        (elif (`self.ActorHasTag` "Purple")
          (set `self.RitimColor` "/Game/Materials/MI_Purple.MI_Purple")
          (set `self.Sound` "/Game/Sounds/S_Degis.S_Degis")
          (set `self.Tag` "Purple")
          (elif (`self.ActorHasTag` "Blue")
            (set `self.RitimColor` "/Game/Materials/MI_BLue.MI_Blue")
            (set `self.Sound` "/Game/Sounds/S_Drum.S_Drum")
            (set `self.Tag` "Blue")
            (elif (`self.ActorHasTag` "Yellow")
              (set `self.RitimColor` "/Game/Materials/MI_Yellow.MI_Yellow")
              (set `self.Sound` "/Game/Sounds/S_Hat.S_Hat")
              (set `self.Tag` "Yellow")
              (elif (`self.ActorHasTag` "Green")
                (set `self.RitimColor` "/Game/Materials/MI_Green.MI_Green")
                (set `self.Sound` "/Game/Sounds/S_Synth.S_Synth")
                (set `self.Tag` "Green")
                (else
                  (set `self.RitimColor` "/Game/Materials/MI_White.MI_White")
                  (set `self.Tag` "Red"))))))))
    (:`then_1`
      (bind _returnvalue (`KismetMaterialLibrary.CreateDynamicMaterialInstance` (`self.RitimColor`)))
      (bind _output_get (set `self.MatInst` _returnvalue))
      (`PrimitiveComponent.SetMaterial` (`self.RitimMesh`) 0 _output_get)
      (`self.Deactivating`))))

(event `self.ActivateTileBP`
  (`self.Activating`))

(event `self.DeactivateTileBP`
  (`self.Deactivating`))

(fn `ActivateAll`
  (bind _outactors (`GameplayStatics.GetAllActorsOfClassWithTag` "/Game/Blueprints/BP_ColorTile.BP_ColorTile_C" (`self.Tag`)))
  (for _array_element _outactors
    (`/Game/Blueprints/BP_ColorTile.Activating` _array_element)))

(fn `Activating`
  (set `self.Opacity` 0.0)
  (`self.SetActorEnableCollision` true)
  (`MaterialInstanceDynamic.SetScalarParameterValue` (`self.MatInst`) "Kenar Boyutları" (`self.Opacity`)))

(fn `DeactivateAll`
  (bind _outactors (`GameplayStatics.GetAllActorsOfClassWithTag` "/Game/Blueprints/BP_ColorTile.BP_ColorTile_C" (`self.Tag`)))
  (for _array_element _outactors
    (`/Game/Blueprints/BP_ColorTile.Deactivating` _array_element)))

(fn `Deactivating`
  (set `self.Opacity` 15.0)
  (`self.SetActorEnableCollision` true)
  (`MaterialInstanceDynamic.SetScalarParameterValue` (`self.MatInst`) "Kenar Boyutları" (`self.Opacity`)))

(fn `Play`
  (if (not (> (`self.Opacity`) 14.0))
    (`GameplayStatics.PlaySound2D` (`self.Sound`) 1.0 1.0 0.0 null null)
    (`self.ActivateAll`)
    (else
      (`self.DeactivateAll`))))

(fn `UserConstructionScript`)