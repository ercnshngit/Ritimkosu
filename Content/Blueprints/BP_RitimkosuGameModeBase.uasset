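; Game mode Blueprint that plays a base sound at start and respawns the player character whenever it is destroyed.
; BeginPlay caches the player character and binds to its OnDestroyed event.
; On destruction it flags the recent death, saves the seconds from the player's Aim, clears all widgets, then spawns and possesses a new character.
; It then calls Respawn to rebind the event, so the cycle repeats.
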(event `Respawn`
  (bind _asbp_player_character (cast `/Game/Blueprints/BP_PlayerCharacter` (`GameplayStatics.GetPlayerCharacter` 0) :!label _label))
  (set `self.Player` _asbp_player_character)
  (add `Actor.OnDestroyed` (`self.Player`) (delegate `OnDestroyed_Event_0`)))

(event `self.ReceiveBeginPlay`
  (`GameplayStatics.PlaySound2D` "/Game/Sounds/base.base" 1.0 1.0 0.0 null null false)
  (goto _label))

(event `OnDestroyed_Event_0`
  (params (DestroyedActor :type "Actor Object Reference"))
  (set `self.bIsPlayerDeadRecently` true)
  (set `self.Time` (`/Game/Widgets/W_Aim.Seconds` (`/Game/Blueprints/BP_PlayerCharacter.Aim` (`self.Player`))))
  (`WidgetLayoutLibrary.RemoveAllWidgets`)
  (bind _returnvalue (`|SpawnActorFromClass` "/Game/Blueprints/BP_PlayerCharacter.BP_PlayerCharacter_C" (`self.Spawn Transform`) "Undefined" "OverrideRootScale" null null))
  (`Controller.Possess` (`GameplayStatics.GetPlayerController` 0) _returnvalue)
  (`self.Respawn`))

(fn `UserConstructionScript`)