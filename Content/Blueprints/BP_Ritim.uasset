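; BP_Ritim is a step-sequencer playhead that triggers BP_RitimTile actors as it moves along a row of tiles.
; A looping one-second timer steps it along X, counting up to TileCount before resetting to its start location.
; After every step, five sphere components each line-trace forward on the Visibility channel and call Play on any BP_RitimTile they hit.
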(event `self.ReceiveBeginPlay`
  (set `self.Default Location` (`SceneComponent.K2_GetComponentLocation` (`self.StaticMesh`)))
  (`KismetSystemLibrary.K2_SetTimer` null "Move" 1.0 true))

(fn `Move`
  (bind _counter (`self.Counter`))
  (`|ExecutionSequence`
    (:`then_0`
      (if (>= (`self.TileCount`) _counter)
        (set `self.Counter` (+ _counter 1))
        (`self.K2_SetActorLocation` (+ (`SceneComponent.K2_GetComponentLocation` (`self.StaticMesh`)) (200.0 0.0 0.0)))
        (else
          (set `self.Counter` 0)
          (`self.K2_SetActorLocation` (`self.Default Location`)))))
    (:`then_1`
      (`self.Play`))))

(fn `Play`
  (bind _sphere1 (`self.Sphere1`))
  (bind _sphere (`self.Sphere`))
  (bind _sphere4 (`self.Sphere4`))
  (bind _sphere3 (`self.Sphere3`))
  (bind _sphere2 (`self.Sphere2`))
  (bind _returnvalue (`SceneComponent.K2_GetComponentLocation` _sphere4))
  (bind _returnvalue_2 (`SceneComponent.K2_GetComponentLocation` _sphere))
  (bind _returnvalue_3 (`SceneComponent.K2_GetComponentLocation` _sphere1))
  (bind _returnvalue_4 (`SceneComponent.K2_GetComponentLocation` _sphere2))
  (bind _returnvalue_5 (`SceneComponent.K2_GetComponentLocation` _sphere3))
  (`|ExecutionSequence`
    (:`then_0`
      (bind _outhit (`KismetSystemLibrary.LineTraceSingle` :`Start` _returnvalue_2 :`End` (+ _returnvalue_2 (* (`SceneComponent.GetForwardVector` _sphere) 500.0)) :`TraceChannel` "TraceTypeQuery1" :`DrawTime` 1.0))
      (bind _asbp_ritim_tile (cast `/Game/Blueprints/BP_RitimTile` (`.HitActor` (`GameplayStatics.BreakHitResult` _outhit))))
      (`/Game/Blueprints/BP_RitimTile.Play` _asbp_ritim_tile))
    (:`then_1`
      (bind _outhit_2 (`KismetSystemLibrary.LineTraceSingle` :`Start` _returnvalue_3 :`End` (+ _returnvalue_3 (* (`SceneComponent.GetForwardVector` _sphere1) 500.0)) :`TraceChannel` "TraceTypeQuery1" :`DrawTime` 1.0))
      (bind _asbp_ritim_tile_2 (cast `/Game/Blueprints/BP_RitimTile` (`.HitActor` (`GameplayStatics.BreakHitResult` _outhit_2))))
      (`/Game/Blueprints/BP_RitimTile.Play` _asbp_ritim_tile_2))
    (:`then_2`
      (bind _outhit_3 (`KismetSystemLibrary.LineTraceSingle` :`Start` _returnvalue_4 :`End` (+ _returnvalue_4 (* (`SceneComponent.GetForwardVector` _sphere2) 500.0)) :`TraceChannel` "TraceTypeQuery1" :`DrawTime` 1.0))
      (bind _asbp_ritim_tile_3 (cast `/Game/Blueprints/BP_RitimTile` (`.HitActor` (`GameplayStatics.BreakHitResult` _outhit_3))))
      (`/Game/Blueprints/BP_RitimTile.Play` _asbp_ritim_tile_3))
    (:`then_3`
      (bind _outhit_4 (`KismetSystemLibrary.LineTraceSingle` :`Start` _returnvalue_5 :`End` (+ _returnvalue_5 (* (`SceneComponent.GetForwardVector` _sphere3) 500.0)) :`TraceChannel` "TraceTypeQuery1" :`DrawTime` 1.0))
      (bind _asbp_ritim_tile_4 (cast `/Game/Blueprints/BP_RitimTile` (`.HitActor` (`GameplayStatics.BreakHitResult` _outhit_4))))
      (`/Game/Blueprints/BP_RitimTile.Play` _asbp_ritim_tile_4))
    (:`then_4`
      (bind _outhit_5 (`KismetSystemLibrary.LineTraceSingle` :`Start` _returnvalue :`End` (+ _returnvalue (* (`SceneComponent.GetForwardVector` _sphere4) 500.0)) :`TraceChannel` "TraceTypeQuery1" :`DrawTime` 1.0))
      (bind _asbp_ritim_tile_5 (cast `/Game/Blueprints/BP_RitimTile` (`.HitActor` (`GameplayStatics.BreakHitResult` _outhit_5))))
      (`/Game/Blueprints/BP_RitimTile.Play` _asbp_ritim_tile_5))))

(fn `UserConstructionScript`)